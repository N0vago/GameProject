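; BP_Skeleton is a 2D flipbook skeleton that attacks on left mouse click and reacts when damaged.
; Both events drive the animation instance through node jumps, to Attack or Hurt.
; A DoOnce gates attacks and resets after a delay of the sprite's flipbook length minus a small margin.
; The damage event only triggers the animation, with no health handling.
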(event Game|Damage|EventAnyDamage
  (params (Damage :type Float%20%28single-precision%29) (DamageType :type Damage%20Type%20Object%20Reference) (InstigatedBy :type Controller%20Object%20Reference) (DamageCauser :type Actor%20Object%20Reference))
  ;[1 1 1] TakingDamage
  (Class|PaperZDAnimInstance|JumptoNode (Variables|/Script/PaperZD.PaperZDAnimationComponent|GetAnimInstance (Variables|Default|GetAnimationComponent)) "Hurt" "None"))

(event Input|MouseEvents|LeftMouseButton
  (params (Key :type Key%20Structure :default "None"))
  ;[1 1 1] Attack
  (:Pressed
    (Utilities|FlowControl|DoOnce false :!label _label
      (:Completed
        (Class|PaperZDAnimInstance|JumptoNode (Variables|/Script/PaperZD.PaperZDAnimationComponent|GetAnimInstance (Variables|Default|GetAnimationComponent)) "Attack" "None")
        (Utilities|FlowControl|Delay (- (Class|PaperFlipbookComponent|GetFlipbookLength (Variables|Default|GetSprite)) 0.1))
        (goto _label Reset)))))

(fn ConstructionScript)