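; BP_Skeleton is a 2D flipbook skeleton enemy that plays attack and hurt animations through PaperZD-style JumpToNode calls.
; HitBox overlap events track whether the player character is inside.
; While overlapping, Tick jumps to Attack through a DoOnce, which resets after a delay just short of the sprite's current flipbook length.
; Any damage received jumps to Hurt; the graph itself neither deals damage nor tracks health.
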(event OnComponentBeginOverlap(HitBox)
  (params (OverlappedComponent :type Primitive%20Component%20Object%20Reference) (OtherActor :type Actor%20Object%20Reference) (OtherComp :type Primitive%20Component%20Object%20Reference) (OtherBodyIndex :type Integer) (bFromSweep :type Boolean) (SweepResult :type Hit%20Result%20Structure%20%28by%20ref%29))
  ;[1 1 1] Attack
  (Utilities|Casting|CastToBP_PlayerCharacter OtherActor)
  (Variables|Default|SetIsOverlapping true))

(event OnComponentEndOverlap(HitBox)
  (params (OverlappedComponent :type Primitive%20Component%20Object%20Reference) (OtherActor :type Actor%20Object%20Reference) (OtherComp :type Primitive%20Component%20Object%20Reference) (OtherBodyIndex :type Integer))
  ;[1 1 1] Attack
  (Utilities|Casting|CastToBP_PlayerCharacter OtherActor)
  (Variables|Default|SetIsOverlapping false))

(event Game|Damage|EventAnyDamage
  (params (Damage :type Float%20%28single-precision%29) (DamageType :type Damage%20Type%20Object%20Reference) (InstigatedBy :type Controller%20Object%20Reference) (DamageCauser :type Actor%20Object%20Reference))
  ;[1 1 1] TakingDamage
  (Class|PaperZDAnimInstance|JumptoNode (Variables|/Script/PaperZD.PaperZDAnimationComponent|GetAnimInstance (Variables|Default|GetAnimationComponent)) "Hurt" "None"))

(event EventTick
  (params (DeltaSeconds :type Float%20%28single-precision%29))
  (if (Variables|Default|GetIsOverlapping)
    (Utilities|FlowControl|DoOnce false :!label _label
      (:Completed
        (Class|PaperZDAnimInstance|JumptoNode (Variables|/Script/PaperZD.PaperZDAnimationComponent|GetAnimInstance (Variables|Default|GetAnimationComponent)) "Attack" "None")
        (Utilities|FlowControl|Delay (- (Class|PaperFlipbookComponent|GetFlipbookLength (Variables|Default|GetSprite)) 0.1))
        (goto _label Reset)))))

(fn ConstructionScript)